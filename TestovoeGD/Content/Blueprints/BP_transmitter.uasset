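; BP_transmitter is a building that siphons resources from the nearest earlier-built house within its radius.
; A sphere overlap collects nearby houses, and EventHouseNubmerFilter keeps those with a lower NumberHouse, targets the nearest and rotates an arrow toward it.
; A self-calling Delay loop then moves one resource per second, idling while the target is invalid or empty and ending once the transmitter is full.
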(event `self.ReceiveBeginPlay`
  (`parent.ReceiveBeginPlay`))

(event `Event_resourse`
  (bind _target (`self.target`))
  ;[1 1 1] Если здание-цель существует, число его ресурсов больше 0, число своих ресурсов меньше 100, то забирай по ресурсу каждую секунду
  (`/Engine/EditorBlueprintResources/StandardMacros.IsValid` _target
    (:`Is Valid`
      (if (> (`/Game/Blueprints/BP_abstract_house.resourse` _target) 0)
        (if (< (`self.resourse`) 100)
          (`/Game/Blueprints/BP_source.Event_minus` _target)
          (`self.Event_plus`)
          (`KismetSystemLibrary.Delay` 1.0 :!label _label)
          (`self.Event_resourse`))
        (else
          (goto _label))))
    (:`Is Not Valid`
      (goto _label))))

(event `Event_plus`
  (set `self.resourse` (+ (`self.resourse`) 1))
  (`self.Event_Text`))

(event `self.Sphere.OnComponentBeginOverlap`
  (params (OverlappedComponent :type "PrimitiveComponent Object Reference") (OtherActor :type "Actor Object Reference") (OtherComp :type "PrimitiveComponent Object Reference") (OtherBodyIndex :type Integer) (bFromSweep :type Boolean) (SweepResult :type "HitResult Structure (by ref)"))
  ;[1 1 1] Получи ссылку на здания в определённом радиусе
  (bind _asbp_abstract_house (cast `/Game/Blueprints/BP_abstract_house` OtherActor))
  ;;[1 1 1] Не реагируй на себя
  (if (not (== _asbp_abstract_house self))
    ;;[1 1 1] Сохрани ссылку на него, если ранее это не было сделано
    (if (not (`KismetArrayLibrary.Array_Contains` (`self.BP_house_all`) _asbp_abstract_house))
      (`KismetArrayLibrary.Array_Add` (`self.BP_house_all`) _asbp_abstract_house))))

(event `self.Event_house_nubmer_filter`
  (bind _scene (`self.Scene`))
  ;[1 1 1] Небольшой костыль. Сохраняем здания построенные ранее, причём в отдельном эвенте.
  (for _array_element (`self.BP_house_all`)
    (if (`KismetArrayLibrary.Array_Contains` (`self.BP_house_number`) _array_element)
      _
      (elif (< (`/Game/Blueprints/BP_abstract_house.number_house` _array_element) (`self.number_house`))
        (`KismetArrayLibrary.Array_Add` (`self.BP_house_number`) _array_element))))
  ;[1 1 1] Получи ссылку на ближайшее здание
  (bind _asbp_abstract_house (cast `/Game/Blueprints/BP_abstract_house` (`.ReturnValue` (`GameplayStatics.FindNearestActor` (`self.K2_GetActorLocation`) (`self.BP_house_number`)))))
  (set `self.target` _asbp_abstract_house)
  ;[1 1 1] Начни выкачивать ресурсы из здания
  (`self.Event_resourse`)
  ;[1 1 1] Доверни стрелку на цель. Если её нет - стрелка скрыта внутри здания
  (`SceneComponent.K2_SetRelativeLocation` _scene (0.0 0.0 90.0) false true)
  (`SceneComponent.K2_SetWorldRotation` _scene (`KismetMathLibrary.FindLookAtRotation` (`SceneComponent.K2_GetComponentLocation` _scene) (`self.K2_GetActorLocation` (`self.target`))) false false))

(fn `UserConstructionScript`
  (`parent.UserConstructionScript`))