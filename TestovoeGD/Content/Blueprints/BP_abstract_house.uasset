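; Abstract base Blueprint for a building that holds a resource count and displays it on a text render.
; BeginPlay refreshes the label and stores the placed location, and a minus event decrements the count and updates the text.
; A teleport event returns the building home when its level number matches the player's, otherwise moves it to a hidden spot where it keeps working.
; The number-filter event is an empty stub.
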(event `Event_house_nubmer_filter`
  ;[1 1 1] см. BP transmitter
)

(event `Event_Text`
  ;[1 1 1] Обновление подписи с ресурсами
  (`TextRenderComponent.K2_SetText` (`self.TextRender`) (`KismetTextLibrary.Conv_IntToText` (`self.resourse`))))

(event `self.ReceiveBeginPlay`
  (`self.Event_Text`)
  ;[1 1 1] Запомни где здание расположили
  (set `self.location_mir` (`self.K2_GetActorLocation`)))

(event `Event_teleport`
  (if (== (`self.LVL_number`) (`/Game/FirstPersonBP/Blueprints/FirstPersonCharacter.LVL_number` (`self.BP_player`)))
    ;[1 1 1] Если здание было установлено в этом мире, то верни его на место
    (`self.K2_SetActorLocation` (`self.location_mir`) false true)
    (else
      ;[1 1 1] Если игрок открывает другой мир, то спрячь здание на другом мини-уровне, где оно продолжит работу
      (`self.K2_SetActorLocation` (`self.location_2`) false true))))

(event `self.ReceiveTick`
  (params (DeltaSeconds :type "Float (single-precision)")))

(event `Event_minus`
  ;[1 1 1] Уменьшение числа ресурсов
  (set `self.resourse` (- (`self.resourse`) 1))
  (`self.Event_Text`))

(fn `UserConstructionScript`)